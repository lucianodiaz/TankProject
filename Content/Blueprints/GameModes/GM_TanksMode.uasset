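; Game mode for a two-team multiplayer tank match, alternating joining players between Red and Blue from a random starting team.
; When enough players join, it spawns and possesses tanks at random team-matched CustomPlayerStarts.
; A looping server timer reapplies team colors and names to pawns.
; It also logs kills, restarts players after a delay and sends end screens when a team is defeated.
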(event Custom|SetColorAndName
  ;[0.2271 1 0 1 32] BeginPlay
  (Networking|SwitchHasAuthority
    (:Authority
      (for _array_element (Variables|Default|GetPCs)
        (Class|ActorsInterface|SetColorTeam(Message) (Pawn|GetControlledPawn _array_element))
        (Class|ActorsInterface|UpdatePlayerName(Message) (Pawn|GetControlledPawn _array_element) (Variables|/Script/Engine.Controller|GetPlayerState _array_element))))))

(event Custom|SpawnPlayers
  (bind _spawnblue (Variables|Default|GetSpawnBlue))
  (for _array_element (Variables|Default|GetPCs)
    (bind _team (Class|StateInterfaces|GetTeam(Message) (Variables|/Script/Engine.Controller|GetPlayerState _array_element)))
    (switch Utilities|FlowControl|Switch|SwitchonETeam _team
      (:NewEnumerator0
        (bind _returnvalue (Game|SpawnActorfromClass "/Game/Blueprints/Player/BP_tank.BP_tank_C" (Transformation|GetActorTransform (Utilities|Array|Get(acopy) (Variables|Default|GetSpawn%20Red) (Math|Random|RandomIntegerinRange 0 (Utilities|RealLength (Variables|Default|GetSpawn%20Red))))) "Undefined" 0 0))
        (Pawn|Possess _array_element _returnvalue))
      (:NewEnumerator1
        (bind _returnvalue_2 (Game|SpawnActorfromClass "/Game/Blueprints/Player/BP_tank.BP_tank_C" (Transformation|GetActorTransform (Utilities|Array|Get(acopy) _spawnblue (Math|Random|RandomIntegerinRange 0 (Utilities|RealLength _spawnblue)))) "Undefined" 0 0))
        (Pawn|Possess _array_element _returnvalue_2)))
    (Utilities|FlowControl|Delay 1.0)
    (CallFunction|SetColorandName)))

(event Custom|FindSpawnPointGM
  ;[1 1 1] Find Point
  (bind _outactors (Actor|GetAllActorsOfClass "/Game/Blueprints/CustomPlayerStart.CustomPlayerStart_C"))
  (for _array_element _outactors
    (switch Utilities|FlowControl|Switch|SwitchonETeam (Variables|/Game/Blueprints/CustomPlayerStart.CustomPlayerStart_C|GetTeam _array_element)
      (:NewEnumerator0
        (Utilities|Array|AddUnique (Variables|Default|GetSpawn%20Red) _array_element))
      (:NewEnumerator1
        (Utilities|Array|AddUnique (Variables|Default|GetSpawnBlue) _array_element)))))

(event EventBeginPlay
  ;[0.2271 1 0 1 32] BeginPlay
  (CallFunction|FindSpawnPointGM)
  (Utilities|Time|SetTimerbyEvent (delegate Custom|SetColorAndName) 0.5 true))

(event EventOnActorKilled
  (params (VictimActor :type Actor%20Object%20Reference) (KillerActor :type Actor%20Object%20Reference))
  (Development|PrintString (Utilities|String|ToString(Text) (Utilities|Text|FormatText "{Killer} has destroyed to {Victim}" (Utilities|GetDisplayName KillerActor) (Utilities|GetDisplayName VictimActor)))))

(event EventPostLogin
  (params (NewPlayer :type Player%20Controller%20Object%20Reference))
  ;[1 0 0.03344 1 34] ON post login
  (Utilities|Array|AddUnique (Variables|Default|GetPCs) NewPlayer)
  (bind _asbp_player_states (Utilities|Casting|CastToBP_PlayerStates (Variables|/Script/Engine.Controller|GetPlayerState NewPlayer)))
  (Variables|/Game/Blueprints/Player/BP_PlayerStates.BP_PlayerStates_C|SetTeam _asbp_player_states (select (Variables|Default|GetTeamBlueSelector) "NewEnumerator1" "NewEnumerator0"))
  (Variables|Default|SetTeamBlueSelector (not (Variables|Default|GetTeamBlueSelector)))
  (CallFunction|SetColorandName)
  (|CallParentFunction NewPlayer))

(event EventGameCompleted
  (params (DefeatedTeam :type ETeam%20Enum :default "NewEnumerator0"))
  ;[1 1 1] GameCompleted
  (Networking|SwitchHasAuthority
    (:Authority
      (for _array_element (Variables|Default|GetPCs)
        (Class|PCsInterface|ShowEndScreen(Message) _array_element DefeatedTeam)))))

(event EventRestartPC
  (params (PC :type Player%20Controller%20Object%20Reference) (CameraDeath :type Pawn%20Object%20Reference))
  ;[1 1 1] Restart player controller
  (Utilities|FlowControl|Delay (Variables|Default|GetWaitResurrection))
  (Class|Pawn|DetachfromControllerPendingDestroy CameraDeath)
  (Actor|SetLifeSpan CameraDeath 2.0)
  (Class|GameModeBase|RestartPlayer PC))

(fn ConstructionScript
  (Variables|Default|SetTeamBlueSelector (Math|Random|RandomBool)))

(fn ReadytoStartMatch
  (if (and (>= (Variables|Default|GetNumPlayers) (Variables|Default|GetMaxPlayerAllowed)) (>= (Utilities|Array|Length (Variables|Default|GetPCs)) (Variables|Default|GetMaxPlayerAllowed)))
    (CallFunction|SpawnPlayers)
    (return (>= (Variables|Default|GetNumPlayers) (Variables|Default|GetMaxPlayerAllowed)))))

(fn ReadytoEndMatch
  (return (Variables|Default|GetIsEndMatch)))

(fn FindPlayerStart
  (params (Player :type Controller%20Object%20Reference) (IncomingName :type String))
  (bind _spawn_red (Variables|Default|GetSpawn%20Red))
  (bind _spawnblue (Variables|Default|GetSpawnBlue))
  (CallFunction|FindSpawnPointGM)
  (bind _team (Class|StateInterfaces|GetTeam(Message) (Variables|/Script/Engine.Controller|GetPlayerState Player)))
  (switch Utilities|FlowControl|Switch|SwitchonETeam _team
    (:NewEnumerator0
      (return (Utilities|Array|Get(acopy) _spawn_red (Math|Random|RandomIntegerinRange 0 (Utilities|RealLength _spawn_red)))))
    (:NewEnumerator1
      (return (Utilities|Array|Get(acopy) _spawnblue (Math|Random|RandomIntegerinRange 0 (Utilities|RealLength _spawnblue)))))))

(fn ChoosePlayerStart
  (params (Player :type Controller%20Object%20Reference))
  (bind _team (Class|StateInterfaces|GetTeam(Message) (Variables|/Script/Engine.Controller|GetPlayerState Player)))
  (switch Utilities|FlowControl|Switch|SwitchonETeam _team
    (:NewEnumerator0
      (return (Utilities|Array|Get(acopy) (Variables|Default|GetSpawn%20Red))))
    (:NewEnumerator1
      (return (Utilities|Array|Get(acopy) (Variables|Default|GetSpawnBlue))))))