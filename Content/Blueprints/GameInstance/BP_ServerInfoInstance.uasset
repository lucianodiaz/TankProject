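; BP_ServerInfoInstance is a game instance Blueprint that handles multiplayer session hosting and joining and exposes team spawn data.
; HostSession creates an advanced session with four public connections, then opens the Test level as a listen server, or prints a message on failure.
; FindSession joins the session result passed to it without running a search.
; Two getters return the stored blue and red spawn values.
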(event EventHostSession
  (|AdvancedSession 0 (Game|GetPlayerController 0) 4 0 false true false true true true false false false true false true
    (:OnSuccess
      (Game|OpenLevel(byName) "Test" true "?listen"))
    (:OnFailure
      (Development|PrintString "Failure"))))

(event EventFindSession
  (params (SessionResult :type Blueprint%20Session%20Result%20Structure))
  (|JoinSession (Game|GetPlayerController 0) SessionResult))

(fn GetBlueSpawn
  (return (Variables|Default|GetSpawnBlue)))

(fn GetRedSpawn
  (return (Variables|Default|GetSpawnRed)))