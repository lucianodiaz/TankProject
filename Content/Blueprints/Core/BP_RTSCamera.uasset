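; RTS camera actor that pans when the mouse cursor nears the edges of the viewport.
; BeginPlay starts two fast looping timers: Left handles both horizontal edges and Up handles both vertical edges.
; Each moves the root by a vector that ramps up across the outer 5% of the screen, scaled by GetCameraSpeed, which grows with spring arm length.
; The SetViewTargetWithBlend call is unwired and never runs.
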(event EventBeginPlay
  (Utilities|Time|SetTimerbyFunctionName 0 "Left" 0.01 true)
  (Utilities|Time|SetTimerbyFunctionName 0 "Up" 0.01 true))

(fn ConstructionScript)

(fn Left
  (bind _returnvalue (Viewport|GetViewportSize))
  (Utilities|FlowControl|Sequence
    (:then_0
      ;[1 1 1] Left
      (bind _returnvalue_2 (Class|WidgetLayoutLibrary|GetMousePositiononViewport))
      (Transformation|AddRelativeLocation (Variables|Default|GetDefaultSceneRoot) (* (Math|Vector|MakeVector 0.0 (CallFunction|GetCameraSpeed -1.0) 0.0) (- 1.0 (Math|Float|Clamp(Float) (Math|Float|NormalizetoRange (.x (* _returnvalue_2 (Class|WidgetLayoutLibrary|GetViewportScale))) 0.0 (* (.x (Viewport|GetViewportSize)) 0.05))))) false false))
    (:then_1
      ;[1 1 1] Right
      (bind _returnvalue_3 (Class|WidgetLayoutLibrary|GetMousePositiononViewport))
      (Transformation|AddRelativeLocation (Variables|Default|GetDefaultSceneRoot) (* (Math|Vector|MakeVector 0.0 (CallFunction|GetCameraSpeed 1.0) 0.0) (Math|Float|Clamp(Float) (Math|Float|NormalizetoRange (.x (* _returnvalue_3 (Class|WidgetLayoutLibrary|GetViewportScale))) (* (.x _returnvalue) 0.95) (.x _returnvalue)))) false false))))

(fn Up
  (bind _returnvalue (Viewport|GetViewportSize))
  (Utilities|FlowControl|Sequence
    (:then_0
      ;[1 1 1] UP
      (bind _returnvalue_2 (Class|WidgetLayoutLibrary|GetMousePositiononViewport))
      (Transformation|AddRelativeLocation (Variables|Default|GetDefaultSceneRoot) (* (Math|Vector|MakeVector (CallFunction|GetCameraSpeed 1.0) 0.0 0.0) (- 1.0 (Math|Float|Clamp(Float) (Math|Float|NormalizetoRange (.y (* _returnvalue_2 (Class|WidgetLayoutLibrary|GetViewportScale))) 0.0 (* (.y (Viewport|GetViewportSize)) 0.05))))) false false))
    (:then_1
      ;[1 1 1] Down
      (bind _returnvalue_3 (Class|WidgetLayoutLibrary|GetMousePositiononViewport))
      (Transformation|AddRelativeLocation (Variables|Default|GetDefaultSceneRoot) (* (Math|Vector|MakeVector (CallFunction|GetCameraSpeed -1.0) 0.0 0.0) (Math|Float|Clamp(Float) (Math|Float|NormalizetoRange (.y (* _returnvalue_3 (Class|WidgetLayoutLibrary|GetViewportScale))) (* (.y _returnvalue) 0.95) (.y _returnvalue)))) false false))))

(fn GetCameraSpeed
  (params (ScaleFactor :type Float%20%28single-precision%29))
  (return (* (+ (* (Math|Float|NormalizetoRange (Variables|/Script/Engine.SpringArmComponent|GetTargetArmLength (Variables|Default|GetSpringArm)) 1e+03 3e+03) 4e+01) 4e+01) ScaleFactor)))