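; Player controller for a multiplayer match with cannon-wielding pawns, linking the pawn, HUD and game mode.
; Looping timers aim the cannon along the mouse ray and track the pawn, possessing a spawned RTS camera and requesting a game mode restart when it is gone.
; Zoom input goes to the pawn.
; Event pairs with CLIENT/Server suffixes relay health, waiting-phase input lock, countdown and end screen to the local player's UI.
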(event Custom|CheckPawn
  (bind _returnvalue (Pawn|GetControlledPawn))
  ;[1 0.04606 0] CheckPawn
  (Utilities|IsValid _returnvalue
    (:Is%20Valid
      (Variables|Default|SetLastPawnLocation (Transformation|GetActorLocation _returnvalue)))
    (:Is%20Not%20Valid
      (bind _returnvalue_2 (Game|SpawnActorfromClass "/Game/Blueprints/Core/BP_RTSCamera.BP_RTSCamera_C" (Math|Transform|MakeTransform (Variables|Default|GetLastPawnLocation)) "Undefined" 0 0))
      (Pawn|Possess _returnvalue_2)
      (CallFunction|OnPawnKilled self _returnvalue_2))))

(event Custom|RotateCannonPC
  (bind (_worldlocation _worlddirection) (Game|Player|ConvertMouseLocationToWorldSpace))
  ;[1 1 1] Rotate Cannon
  (if (Pawn|IsLocalController)
    (Class|ActorsInterface|RotateCannon(Message) (Pawn|GetControlledPawn) _worldlocation _worlddirection)))

(event Custom|WaitingPlayersCLIENT
  ;[1 1 1] WaitingPlayers
  (Input|DisableInput self))

(event Custom|AddEndScreenServer
  (params (TeamDefeated :type ETeam%20Enum :default "NewEnumerator0"))
  ;[1 0 0.8855] Show end Screen Replicated
  (CallFunction|AddEndScreenClient TeamDefeated))

(event Custom|UpdateHealthBarCLIENT
  (params (Health :type Float%20%28single-precision%29))
  ;[1 1 1] UPDATE HEALTHBAR
  (Class|BPIUIInterface|UpdateHealthBar(Message) (Variables|Default|GetGUI) Health))

(event Custom|AddEndScreenClient
  (params (TeamDefeated :type ETeam%20Enum :default "NewEnumerator0"))
  ;[1 0 0.8855] Show end Screen Replicated
  (bind _returnvalue (UserInterface|CreateWidget "/Game/Widget/Player/BPW_EndGame.BPW_EndGame_C" 0 TeamDefeated))
  (UserInterface|Viewport|AddtoViewport _returnvalue 0)
  (Input|SetInputModeUIOnly self _returnvalue "DoNotLock"))

(event Custom|PreparingMatchCLIENT
  (Input|EnableInput self)
  (Utilities|IsValid (Variables|Default|GetGUI)
    (:Is%20Valid
      (Class|BPIUIInterface|UpdateOverlay(Message) (Variables|Default|GetGUI)))))

(event Custom|UpdateTimerToStartCLIENT
  (params (NewParam :type Integer))
  (Utilities|IsValid (Variables|Default|GetGUI)
    (:Is%20Valid
      (Class|BPIUIInterface|UpdateTimer(Message) (Variables|Default|GetGUI) NewParam))))

(event EventBeginPlay
  ;[0.1194 1 0] Beginplay
  (Utilities|Time|SetTimerbyFunctionName 0 "RotateCannonPC" 0.01 true)
  (Utilities|Time|SetTimerbyEvent (delegate Custom|CheckPawn) 0.1 true)
  (if (Pawn|IsLocalController)
    (bind _returnvalue (UserInterface|CreateWidget "/Game/Widget/Player/BPW_GUI.BPW_GUI_C" self))
    (bind _output_get (Variables|Default|SetGUI _returnvalue))
    (UserInterface|Viewport|AddtoViewport _output_get 0)))

(event EventOnPawnKilled
  (params (PC :type Player%20Controller%20Object%20Reference) (CameraDeath :type Pawn%20Object%20Reference))
  ;[1 1 1] onPawn Killed
  (Class|GameModeInterface|RestartPC(Message) (Game|GetGameMode) PC CameraDeath))

(event EventShowEndScreen
  (params (TeamDefeated :type ETeam%20Enum :default "NewEnumerator2"))
  ;[1 0 0.8855] Show end Screen Replicated
  (Networking|SwitchHasAuthority
    (:Authority
      (CallFunction|AddEndScreenServer TeamDefeated))))

(event EventGetHit
  (params (Health :type Float%20%28single-precision%29))
  ;[1 1 1] UPDATE HEALTHBAR
  (CallFunction|UpdateHealthBarCLIENT Health))

(event EventWaitingPlayers
  ;[1 1 1] WaitingPlayers
  (CallFunction|WaitingPlayersCLIENT))

(event EventPreparingMatch
  (CallFunction|PreparingMatchCLIENT))

(event EventUpdateTimertoStart
  (params (NewParam :type Integer))
  (CallFunction|UpdateTimertoStartCLIENT NewParam))

(event Input|AxisEvents|InputAxisZoom
  (params (AxisValue :type Float%20%28single-precision%29))
  ;[1 1 1] Zoom
  (if (Pawn|IsLocalController)
    (Class|ActorsInterface|CameraZoom(Message) (Pawn|GetControlledPawn) AxisValue)))

(fn ConstructionScript)