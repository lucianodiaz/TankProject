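; Player-controlled multiplayer tank with team colors, a cannon, camera zoom and an overhead health and name widget.
; Turret aim runs from a trace through server and multicast events to smoothed yaw; shots spawn BP_Bullet on the server, with a timer gating fire rate.
; PlayerState team sets HealthComponent team and a RepNotify color, while team also selects the capsule collision profile.
; Death launches body and turret as physics debris, then detaches the controller.
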(event OnHealthChanged(HealthComponent)
  (params (DamagedActor :type Actor%20Object%20Reference) (Damage :type Float%20%28single-precision%29) (DeltaDamage :type Float%20%28single-precision%29) (DamageType :type Damage%20Type%20Object%20Reference) (InstigatedBy :type Controller%20Object%20Reference) (DamageCauser :type Actor%20Object%20Reference) (isDied :type Boolean))
  (if (== DeltaDamage 1.0)
    (Utilities|FlowControl|Delay 1.0))
  (Class|PCsInterface|GetHit(Message) (Game|GetInstigatorController) DeltaDamage))

(event Custom|FirePrimary
  (bind _pointshoot (Variables|Default|GetPointShoot))
  ;[1 0 0.6559 1 94] Fire Replicated
  (if (not (Ability|HasAuthority))
    (CallFunction|ServerFirePrimary)
    (else
      (Game|SpawnActorfromClass "/Game/Blueprints/BP_Bullet.BP_Bullet_C" (Math|Transform|MakeTransform (Transformation|GetWorldLocation _pointshoot) (Transformation|GetWorldRotation _pointshoot) "1,1,1") "AlwaysSpawn" self 0)
      (Variables|Default|SetLastFireTime (Utilities|Time|GetTimeSeconds)))))

(event Custom|ServerFirePrimary
  ;[1 0 0.6559 1 94] Fire Replicated
  (CallFunction|FirePrimary))

(event Custom|UpdateHealthBarMULTI
  (params (NewParam :type Float%20%28single-precision%29))
  ;[1 0 0.6249 1 49] Update HealthBar Replicated
  (Class|BPIUIInterface|UpdateHealthBar(Message) (UserInterface|GetUserWidgetObject (Variables|Default|GetHealthBar)) NewParam))

(event Custom|UpdatePlayerNameMULTI
  (params (state :type Player%20State%20Object%20Reference))
  ;[1 1 1] Update PLAYERNAME
  (Utilities|IsValid state
    (:Is%20Valid
      (Class|BPIUIInterface|UpdatePlayerName(Message) (UserInterface|GetUserWidgetObject (Variables|Default|GetHealthBar)) (Utilities|Text|ToText(String) (PlayerState|GetPlayerName state))))))

(event Custom|RotateCannonSERVER
  (params (NewParam :type Vector) (NewParam2 :type Vector))
  ;[1 0 0.8298 1 94] Rotate Cannon  Replicated
  ;;[0.3645 1 0] First pass
  (CallFunction|RotateCannonLocally NewParam NewParam2))

(event Custom|SetCollisionMULTI
  (params (Target :type Primitive%20Component%20Object%20Reference) (InCollisionProfileName :type Name))
  ;[0 1 0.2559 1 47] Begin play
  (Collision|SetCollisionProfileName Target InCollisionProfileName true :!class /Script/Engine.PrimitiveComponent))

(event Custom|RotateCannonLocally
  (params (WorldLocation :type Vector) (WorldDirection :type Vector))
  ;[1 0 0.8298 1 94] Rotate Cannon  Replicated
  ;;[0.1134 1 0] Seccond Pass
  (bind _outhit (Collision|LineTraceByChannel WorldLocation (+ WorldDirection (* WorldDirection (+ (Variables|/Script/Engine.SpringArmComponent|GetTargetArmLength (Variables|Default|GetSpringArm)) 1e+04))) "TraceTypeQuery1" false 0 "None"))
  (CallFunction|RotateCannonLocallyMULTI (.location _outhit)))

(event Custom|RotateCannonLocallyMULTI
  (params (Target :type Vector))
  (bind _turret (Variables|Default|Getturret))
  (bind _returnvalue (Transformation|GetWorldLocation _turret))
  (bind _returnvalue_2 (Math|Rotator|FindLookatRotation _returnvalue Target))
  ;[1 0 0.8298 1 94] Rotate Cannon  Replicated
  ;;[0.1277 1 0] Third Pass
  (if (!= (.yaw (Transformation|GetWorldRotation (Variables|Default|Getturret))) (.yaw _returnvalue_2))
    (Transformation|SetWorldRotation (Variables|Default|Getturret) (Math|Interpolation|RInterpTo (Transformation|GetWorldRotation (Variables|Default|Getturret)) (Math|Rotator|MakeRotator 0.0 0.0 (.yaw _returnvalue_2)) (Utilities|Time|GetWorldDeltaSeconds) 7.0) false false)))

(event EventGetHit
  (params (DamagedAmmount :type Float%20%28single-precision%29))
  ;[1 0 0.6249 1 49] Update HealthBar Replicated
  (Networking|SwitchHasAuthority
    (:Authority
      (CallFunction|UpdateHealthBarMULTI DamagedAmmount))))

(event EventSetColorTeam
  ;[0.6823 1 0.3646 1 85] SET COLOR
  (Networking|SwitchHasAuthority
    (:Authority
      (bind _asbp_player_states (Utilities|Casting|CastToBP_PlayerStates (Variables|GetPlayerState)))
      (Variables|/Game/Blueprints/Components/BP_HealthComponent.BP_HealthComponent_C|SetTeam (Variables|Default|GetHealthComponent) (Variables|/Game/Blueprints/Player/BP_PlayerStates.BP_PlayerStates_C|GetTeam _asbp_player_states))
      (switch Utilities|FlowControl|Switch|SwitchonETeam (Variables|/Game/Blueprints/Player/BP_PlayerStates.BP_PlayerStates_C|GetTeam _asbp_player_states)
        (:NewEnumerator0
          (Variables|Default|SetColorTeam "1.000000, 0, 0"))
        (:NewEnumerator1
          (Variables|Default|SetColorTeam "0, 0,1.000000"))))))

(event EventRotateCannon
  (params (WorldLocation :type Vector :default "0, 0, 0") (WorldDirection :type Vector :default "0, 0, 0"))
  ;[1 0 0.8298 1 94] Rotate Cannon  Replicated
  ;;[0.3645 1 0] First pass
  (Networking|SwitchHasAuthority
    (:Authority
      (CallFunction|RotateCannonLocally WorldLocation WorldDirection))
    (:Remote
      (CallFunction|RotateCannonSERVER WorldLocation WorldDirection))))

(event EventBeginPlay
  ;[0 1 0.2559 1 47] Begin play
  (Utilities|FlowControl|Sequence
    (:then_0
      (Variables|Default|SetTimeBetweenShoots (/ 6e+01 (Variables|Default|GetRateOfFire)))
      (Class|BPIUIInterface|UpdateHealthBar(Message) (UserInterface|GetUserWidgetObject (Variables|Default|GetHealthBar)) (Default|GetHealth (Variables|Default|GetHealthComponent))))
    (:then_1
      (Utilities|FlowControl|Delay 1.0)
      (CallFunction|SetCollisionMULTI (Variables|Collision|GetCapsuleComponent) (Utilities|Select :Index (Variables|/Game/Blueprints/Components/BP_HealthComponent.BP_HealthComponent_C|GetTeam (Variables|Default|GetHealthComponent)) :NewEnumerator2 "BlockAll" :NewEnumerator0 "RedCollision" :NewEnumerator1 "BlueCollision")))))

(event EventUpdatePlayerName
  (params (PlayerState :type Player%20State%20Object%20Reference))
  ;[1 1 1] Update PLAYERNAME
  (Networking|SwitchHasAuthority
    (:Authority
      (CallFunction|UpdatePlayerNameMULTI PlayerState))))

(event EventIsDead
  ;[0 0 0] IS DEAD
  (if (not (Variables|Default|GetbIsDied))
    (Components|Movement|StopMovementImmediately (Pawn|GetMovementComponent))
    (|EffectDestroyCannon)
    (CallFunction|DeathEffectBody)
    (Actor|SetLifeSpan 4.0)
    (Collision|SetCollisionEnabled (Variables|Collision|GetCapsuleComponent) "NoCollision")
    (Utilities|FlowControl|Delay 1.0)
    (Class|Pawn|DetachfromControllerPendingDestroy)))

(event EventCameraZoom
  (params (AxisValue :type Float%20%28single-precision%29))
  ;[1 1 1] Camera zoom
  (bind _output_get (Variables|Default|SetZoomFactor (Math|Float|Clamp(Float) (+ (Variables|Default|GetZoomFactor) (* AxisValue -1.0)) 0.0 1e+01)))
  (Variables|/Script/Engine.SpringArmComponent|SetTargetArmLength (Variables|Default|GetSpringArm) (+ (* _output_get 1e+02) 8e+02)))

(event Input|ActionEvents|InputActionPrimaryShoot
  (params (Key :type Key%20Structure :default "None"))
  ;[1 0 0.6559 1 94] Fire Replicated
  (:Pressed
    (CallFunction|StartPrimaryFire)))

(event Input|AxisEvents|InputAxisForward
  (params (AxisValue :type Float%20%28single-precision%29))
  ;[1 0 0.5714 1 47] Movement
  (Pawn|Input|AddMovementInput (Math|Vector|GetForwardVector (Pawn|GetControlRotation :!class /Script/Engine.Pawn)) AxisValue false))

(event Input|AxisEvents|InputAxisRight
  (params (AxisValue :type Float%20%28single-precision%29))
  ;[1 0 0.5714 1 47] Movement
  (Pawn|Input|AddControllerYawInput (* AxisValue (Variables|Default|GetBaseYawRotation) (Utilities|Time|GetWorldDeltaSeconds))))

(fn ConstructionScript)

(fn StartPrimaryFire
  (if (not (Variables|Default|GetbIsShooting))
    (Variables|Default|SetbIsShooting true)
    (CallFunction|FirePrimary)
    (bind _returnvalue (Utilities|Time|SetTimerbyFunctionName 0 "StopPrimaryFire" (Variables|Default|GetTimeBetweenShoots) true))
    (Variables|Default|SetFireTimerHandle _returnvalue)))

(fn StopPrimaryFire
  (Variables|Default|SetbIsShooting false))

(fn OnRepTeam
  (switch Utilities|FlowControl|Switch|SwitchonETeam (Variables|Default|GetTeam)
    (:NewEnumerator0
      (Rendering|Material|SetVectorParameterValueonMaterials (Variables|Default|GetBody) "color" "0, 0, 0"))
    (:NewEnumerator1
      (Rendering|Material|SetVectorParameterValueonMaterials (Variables|Default|GetBody) "color" "0.000000,0.000000,1.000000"))))

(fn OnRepColorTeam
  (Rendering|Material|SetVectorParameterValueonMaterials (Variables|Default|GetBody) "color" (Variables|Default|GetColorTeam)))

(fn DeathEffectBody
  (bind _returnvalue (Math|Random|RandomFloatinRange -5e+01 5e+01))
  (bind _body (Variables|Default|GetBody))
  (Physics|AddImpulse _body (Math|Vector|MakeVector _returnvalue _returnvalue 4e+03) "None" false)
  (Transformation|AddWorldRotation _body (Math|Interpolation|RInterpTo (Transformation|GetWorldRotation _body) (Math|Random|RandomRotator false) 1.0 0.5) false false))

(fn GetNickname
  (params (Character :type Character%20Object%20Reference))
  (return (PlayerState|GetPlayerName (Variables|/Script/Engine.Pawn|GetPlayerState Character))))

(fn GetPlayerName
  (bind _playerstate (Variables|GetPlayerState))
  (bind _returnvalue (PlayerState|GetPlayerName _playerstate))
  (return (Utilities|String|SelectString "Map" _returnvalue (Utilities|Enum|Equal(Enum) _returnvalue ""))))

(fn GetTeam
  (return (Variables|/Game/Blueprints/Components/BP_HealthComponent.BP_HealthComponent_C|GetTeam (Variables|Default|GetHealthComponent))))