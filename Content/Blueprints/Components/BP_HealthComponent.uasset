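; Health component that tracks damage and death for its owning actor in a team-based tank game.
; It binds to the owner's any-damage event and accepts damage only from BP_tank causers on another team, unless invulnerable.
; Each hit clamps Health, prints it, fires a health-changed call and reports kills to the game mode.
; Health's RepNotify messages the owner with the health fraction and death.
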(event Custom|HandleTakeAnyDamage
  (params (DamagedActor :type Actor%20Object%20Reference) (Damage :type Float%20%28single-precision%29) (DamageType :type Damage%20Type%20Object%20Reference) (InstigatedBy :type Controller%20Object%20Reference) (DamageCauser :type Actor%20Object%20Reference))
  (Utilities|IsValid DamagedActor
    (:Is%20Valid
      (bind _asbp_tank (Utilities|Casting|CastToBP_tank DamageCauser))
      (if (not (Variables|Default|GetIsInvulnerable))
        (if (and (> Damage 0.0) (Utilities|Enum|NotEqual(Enum) (Variables|Default|GetTeam) (Variables|/Game/Blueprints/Player/BP_PlayerStates.BP_PlayerStates_C|GetTeam (.AsBP%20Player%20States (Utilities|Casting|CastToBP_PlayerStates (Variables|/Script/Engine.Pawn|GetPlayerState _asbp_tank))))))
          (bind _output_get (Variables|Default|SetHealth (Math|Float|Clamp(Float) (- (Variables|Default|GetHealth) Damage) 0.0 (Variables|Default|GetDefaultHealth))))
          (Variables|Default|SetbIsDied (<= _output_get 0.0))
          (Development|PrintString (Utilities|String|ToString(Text) (Utilities|Text|FormatText "Health is {Health}" _output_get)))
          (Default|CallOnHealthChanged DamagedActor Damage (Math|Float|Clamp(Float) (- (Variables|Default|GetHealth) Damage) 0.0 (Variables|Default|GetDefaultHealth)) DamageType InstigatedBy DamageCauser)
          (if (Variables|Default|GetbIsDied)
            (Class|GameModeInterface|OnActorKilled(Message) (Game|GetGameMode) DamagedActor DamageCauser)))))))

(event EventBeginPlay
  (Utilities|FlowControl|Sequence
    (:then_0
      (Variables|Default|SetHealth (Variables|Default|GetDefaultHealth)))
    (:then_1
      (if (Utilities|IsValid (Components|GetOwner))
        (EventDispatchers|BindEventtoOnTakeAnyDamage (Components|GetOwner) (delegate Custom|HandleTakeAnyDamage))))))

(fn GetHealth
  (return (Variables|Default|GetHealth)))

(fn OnRepHealth
  (bind _returnvalue (Components|GetOwner))
  (if (<= (Variables|Default|GetHealth) 0.0)
    (Class|ActorsInterface|GetHit(Message) _returnvalue 0.0)
    (Class|ActorsInterface|IsDead(Message) _returnvalue)
    (else
      (Class|ActorsInterface|GetHit(Message) (Components|GetOwner) (/ (Variables|Default|GetHealth) (Variables|Default|GetDefaultHealth))))))