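; BP_Nexus is a team objective structure whose death decides the match.
; One second after BeginPlay it sets its static mesh collision to BlockAll.
; When its father object is destroyed, it removes the health component's invulnerability, opening it to damage.
; On death it passes its team to the game mode's game-completed message before running the parent death logic.
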(event EventBeginPlay
  (|CallParentFunction)
  (Utilities|FlowControl|Delay 1.0)
  (Collision|SetCollisionProfileName (Variables|Default|GetStaticMesh) "BlockAll" true :!class /Script/Engine.PrimitiveComponent))

(event Collision|EventActorBeginOverlap
  (params (OtherActor :type Actor%20Object%20Reference)))

(event EventTick
  (params (DeltaSeconds :type Float%20%28single-precision%29)))

(event EventIsDead
  (Class|GameModeInterface|GameCompleted(Message) (Game|GetGameMode) (Variables|/Game/Blueprints/Components/BP_HealthComponent.BP_HealthComponent_C|GetTeam (Variables|Default|GetHealthComponent)))
  (|CallParentFunction))

(event EventOnFatherDestroyed
  (Variables|/Game/Blueprints/Components/BP_HealthComponent.BP_HealthComponent_C|SetIsInvulnerable (Variables|Default|GetHealthComponent) false))

(fn ConstructionScript
  (|CallParentFunction))