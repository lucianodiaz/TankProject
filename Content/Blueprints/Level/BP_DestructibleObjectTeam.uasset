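; BP_DestructibleObjectTeam is a team-owned destructible object with a health bar widget.
; On BeginPlay it passes its team to the HealthComponent, tints the mesh red or blue, and initializes the bar from the health ratio.
; Hits update the bar on the authority and call UpdateHealthBarMULTI to update it again, apparently as a multicast.
; On death it notifies any valid ChildObject that its parent was destroyed, then destroys itself.
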(event Custom|UpdateHealthBarMULTI
  (params (NewParam :type Float%20%28single-precision%29))
  (Class|BPIUIInterface|UpdateHealthBar(Message) (UserInterface|GetUserWidgetObject (Variables|Default|GetWidget)) NewParam))

(event EventBeginPlay
  (bind _healthcomponent (Variables|Default|GetHealthComponent))
  (Variables|/Game/Blueprints/Components/BP_HealthComponent.BP_HealthComponent_C|SetTeam (Variables|Default|GetHealthComponent) (Variables|Default|GetTeam))
  (Utilities|FlowControl|Sequence
    (:then_0
      (switch Utilities|FlowControl|Switch|SwitchonETeam (Variables|Default|GetTeam)
        (:NewEnumerator0
          (Rendering|Material|SetVectorParameterValueonMaterials (Variables|Default|GetStaticMesh) "color" "1.000000,0.000000, 0"))
        (:NewEnumerator1
          (Rendering|Material|SetVectorParameterValueonMaterials (Variables|Default|GetStaticMesh) "color" "0.000000,0.000000,1.000000"))))
    (:then_1
      (Class|BPIUIInterface|UpdateHealthBar(Message) (UserInterface|GetUserWidgetObject (Variables|Default|GetWidget)) (/ (Default|GetHealth _healthcomponent) (Variables|/Game/Blueprints/Components/BP_HealthComponent.BP_HealthComponent_C|GetDefaultHealth _healthcomponent))))))

(event EventIsDead
  (bind _childobject (Variables|Default|GetChildObject))
  (Utilities|IsValid _childobject
    (:Is%20Valid
      (Default|OnFatherDestroyed _childobject)
      (Actor|DestroyActor))
    (:Is%20Not%20Valid
      (Actor|DestroyActor))))

(event EventGetHit
  (params (DamagedAmmount :type Float%20%28single-precision%29))
  (Networking|SwitchHasAuthority
    (:Authority
      (Class|BPIUIInterface|UpdateHealthBar(Message) (UserInterface|GetUserWidgetObject (Variables|Default|GetWidget)) DamagedAmmount)
      (CallFunction|UpdateHealthBarMULTI DamagedAmmount))))

(fn ConstructionScript)