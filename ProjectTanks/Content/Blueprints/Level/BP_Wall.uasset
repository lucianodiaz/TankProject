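; BP_Wall is a level wall that removes itself once enough of its pillars have been destroyed.
; Each OnFatherDestroyed event increments a destroyed-pillar counter, and reaching the default pillar count destroys the wall after a short delay.
; On BeginPlay it runs the parent logic and hides its Widget.
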(event EventBeginPlay
  (|CallParentFunction)
  (Rendering|SetVisibility (Variables|Default|GetWidget) false false))

(event Collision|EventActorBeginOverlap
  (params (OtherActor :type Actor%20Object%20Reference)))

(event EventTick
  (params (DeltaSeconds :type Float%20%28single-precision%29)))

(event EventOnFatherDestroyed
  (Variables|Default|SetDestroyedPillarNumber (+ (Variables|Default|GetDestroyedPillarNumber) 1))
  (if (>= (Variables|Default|GetDestroyedPillarNumber) (Variables|Default|GetDefaultPillarNumber))
    (Utilities|FlowControl|Delay 1.0)
    (Actor|DestroyActor)))

(fn ConstructionScript
  (|CallParentFunction))