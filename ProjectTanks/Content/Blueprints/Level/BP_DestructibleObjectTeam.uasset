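; BP_DestructibleObjectTeam is a team-owned destructible level object, colored red or blue by its team.
; On BeginPlay it copies its Team to the HealthComponent and sets the static mesh's "color" material parameter to match.
; When the IsDead event fires with a valid ChildObject, it calls DestroyedObject on that object and then destroys itself.
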(event EventBeginPlay
  (Variables|/Game/Blueprints/BP_HealthComponent.BP_HealthComponent_C|SetTeam (Variables|Default|GetHealthComponent) (Variables|Default|GetTeam))
  (switch Utilities|FlowControl|Switch|SwitchonETeam (Variables|Default|GetTeam)
    (:NewEnumerator0
      (Rendering|Material|SetVectorParameterValueonMaterials (Variables|Default|GetStaticMesh) "color" "1.000000,0.000000, 0"))
    (:NewEnumerator1
      (Rendering|Material|SetVectorParameterValueonMaterials (Variables|Default|GetStaticMesh) "color" "0.000000,0.000000,1.000000"))))

(event EventIsDead
  (bind _childobject (Variables|Default|GetChildObject))
  (Utilities|IsValid _childobject
    (:Is%20Valid
      (Default|DestroyedObject _childobject)
      (Actor|DestroyActor))))

(fn ConstructionScript)