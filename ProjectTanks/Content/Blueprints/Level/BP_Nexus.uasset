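; BP_Nexus is a team-owned Nexus structure that reports its destruction to the game mode.
; When OnFatherDestroyed fires, it clears the invulnerability flag on its HealthComponent so it can be damaged.
; Its IsDead event passes the HealthComponent's team to NexusDestroyedMessage on the game mode, then runs the parent's death logic.
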(event EventBeginPlay
  (|CallParentFunction) ; This node is disabled and will not be called.\nDrag off pins to build functionality.
)

(event Collision|EventActorBeginOverlap
  (params (OtherActor :type Actor%20Object%20Reference)))

(event EventTick
  (params (DeltaSeconds :type Float%20%28single-precision%29)))

(event EventIsDead
  (Class|GameModeInterface|NexusDestroyed(Message) (Game|GetGameMode) (Variables|/Game/Blueprints/BP_HealthComponent.BP_HealthComponent_C|GetTeam (Variables|Default|GetHealthComponent)))
  (|CallParentFunction))

(event EventOnFatherDestroyed
  (Variables|/Game/Blueprints/BP_HealthComponent.BP_HealthComponent_C|SetIsInvulnerable (Variables|Default|GetHealthComponent) false))

(fn ConstructionScript
  (|CallParentFunction))