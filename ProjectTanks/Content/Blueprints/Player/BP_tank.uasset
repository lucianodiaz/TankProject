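; Player-controlled tank pawn that drives along its control rotation, turns by yaw input and fires bullets.
; On BeginPlay it links its health bar widget and copies the team from the player state into its health component.
; Each press fires one shot, relayed to the server to spawn BP_Bullet, with a looping timer clearing the shooting flag as a rate-of-fire cooldown.
; Hold-to-autofire and timer-clearing logic is present but disconnected.
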(event Custom|FirePrimary
  (if (not (Ability|HasAuthority))
    (CallFunction|ServerFirePrimary)
    (else
      (Game|SpawnActorfromClass "/Game/Blueprints/BP_Bullet.BP_Bullet_C" (Math|Transform|MakeTransform (Transformation|GetWorldLocation (Variables|Default|GetPointShoot)) (Transformation|GetActorRotation) "1,1,1") "AlwaysSpawn" self 0)
      (Variables|Default|SetLastFireTime (Utilities|Time|GetTimeSeconds)))))

(event Custom|ServerFirePrimary
  (CallFunction|FirePrimary))

(event EventBeginPlay
  (Variables|Default|SetTimeBetweenShoots (/ 6e+01 (Variables|Default|GetRateOfFire)))
  (bind _asbpw_health_bar (Utilities|Casting|CastToBPW_HealthBar (UserInterface|GetUserWidgetObject (Variables|Default|GetWidget))))
  (Variables|/Game/Widget/BPW_HealthBar.BPW_HealthBar_C|SetPawnRef _asbpw_health_bar self)
  (bind _asbp_player_states (Utilities|Casting|CastToBP_PlayerStates (Variables|GetPlayerState)))
  (bind _output_get (Variables|Default|SetTeam (Variables|/Game/Blueprints/Player/BP_PlayerStates.BP_PlayerStates_C|GetTeam _asbp_player_states)))
  (Variables|/Game/Blueprints/BP_HealthComponent.BP_HealthComponent_C|SetTeam (Variables|Default|GetHealthComponent) _output_get))

(event Input|ActionEvents|InputActionPrimaryShoot
  (params (Key :type Key%20Structure :default "None"))
  (:Pressed
    (CallFunction|StartPrimaryFire)))

(event Input|AxisEvents|InputAxisForward
  (params (AxisValue :type Float%20%28single-precision%29))
  ;[1 1 1] Movement
  (Pawn|Input|AddMovementInput (Math|Vector|GetForwardVector (Pawn|GetControlRotation :!class /Script/Engine.Pawn)) AxisValue false))

(event Input|AxisEvents|InputAxisRight
  (params (AxisValue :type Float%20%28single-precision%29))
  ;[1 1 1] Movement
  (Pawn|Input|AddControllerYawInput AxisValue))

(fn ConstructionScript)

(fn StartPrimaryFire
  (if (not (Variables|Default|GetbIsShooting))
    (Variables|Default|SetbIsShooting true)
    (CallFunction|FirePrimary)
    (bind _returnvalue (Utilities|Time|SetTimerbyFunctionName 0 "StopPrimaryFire" (Variables|Default|GetTimeBetweenShoots) true))
    (Variables|Default|SetFireTimerHandle _returnvalue)))

(fn StopPrimaryFire
  (Variables|Default|SetbIsShooting false))