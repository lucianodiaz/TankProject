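; Actor component that gives its owner health and reports when that health runs out.
; On BeginPlay it binds to the owner's OnTakeAnyDamage and sets Health to DefaultHealth.
; Positive damage lowers Health within zero and DefaultHealth unless IsInvulnerable is set, then prints the value.
; Health's RepNotify sends the IsDead interface message to the owner at zero, leaving the death response to that actor.
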(event Custom|HandleTakeAnyDamage
  (params (DamagedActor :type Actor%20Object%20Reference) (Damage :type Float%20%28single-precision%29) (DamageType :type Damage%20Type%20Object%20Reference) (InstigatedBy :type Controller%20Object%20Reference) (DamageCauser :type Actor%20Object%20Reference))
  (if (not (Variables|Default|GetIsInvulnerable))
    (if (> Damage 0.0)
      (bind _output_get (Variables|Default|SetHealth (Math|Float|Clamp(Float) (- (Variables|Default|GetHealth) Damage) 0.0 (Variables|Default|GetDefaultHealth))))
      (Development|PrintString (Utilities|String|ToString(Text) (Utilities|Text|FormatText "Health is {Health}" _output_get))))))

(event EventBeginPlay
  (Utilities|FlowControl|Sequence
    (:then_0
      (if (Utilities|IsValid (Components|GetOwner))
        (EventDispatchers|BindEventtoOnTakeAnyDamage (Components|GetOwner) (delegate Custom|HandleTakeAnyDamage))))
    (:then_1
      (Variables|Default|SetHealth (Variables|Default|GetDefaultHealth)))))

(fn GetHealth
  (return (Variables|Default|GetHealth)))

(fn OnRepHealth
  (if (<= (Variables|Default|GetHealth) 0.0)
    (Class|GeneralInterface|IsDead(Message) (Components|GetOwner))))